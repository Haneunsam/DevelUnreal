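; BP_Item is a pickup that drifts toward the player and raises their level when collected.
; Each Tick, while the player is under 500 units away, it lerps its Sphere toward the pawn using DeltaSeconds as alpha.
; When the actor location nearly matches the pawn's, it increments Level on BP_Player_State and destroys itself.
; The overlap event's movement offset is multiplied by zero, and MoveToPlayer is empty.
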(event `self.ReceiveTick`
  (params (DeltaSeconds :type "Float (single-precision)"))
  (bind _returnvalue (`self.K2_GetActorLocation`))
  (bind _returnvalue_2 (`self.K2_GetActorLocation` (`GameplayStatics.GetPlayerPawn` 0)))
  (if (not (<= 500.0 (`KismetMathLibrary.Vector_Distance` _returnvalue _returnvalue_2)))
    (`SceneComponent.K2_SetWorldLocation` (`self.Sphere`) (`KismetMathLibrary.VLerp` _returnvalue _returnvalue_2 DeltaSeconds) false false)
    (if (== _returnvalue _returnvalue_2 :`ErrorTolerance` 100.0)
      (bind _asbp_player_state (cast `/Game/1_Blueprints/BP_Player_State` (`GameplayStatics.GetPlayerState` 0)))
      (set `/Game/1_Blueprints/BP_Player_State.Level` (+ (`/Game/1_Blueprints/BP_Player_State.Level` _asbp_player_state) 1) _asbp_player_state)
      (`self.K2_DestroyActor`))))

(event `self.ReceiveActorBeginOverlap`
  (params (OtherActor :type "Actor Object Reference"))
  (`SceneComponent.K2_AddWorldOffset` (`self.Sphere`) (* (* (`KismetMathLibrary.Normal` (- (`self.K2_GetActorLocation` (`GameplayStatics.GetPlayerPawn` 0)) (`self.K2_GetActorLocation`))) (`self.Speed`)) (0.0 0.0 0.0)) false false))

(fn `Move_to_Player`)

(fn `UserConstructionScript`)