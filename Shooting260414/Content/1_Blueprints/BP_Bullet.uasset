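; BP_Bullet is a projectile that flies forward at constant speed and damages what it overlaps.
; Each tick sweeps the Box component along its forward vector.
; Cube overlaps apply fixed damage to any actor except the owner, while an actor overlap with BP_Enemy spawns a scaled-up hit particle system and destroys the bullet.
; A timer-based self-destruct is disconnected, so only enemy overlaps destroy it here.
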(event `self.ReceiveTick`
  (params (DeltaSeconds :type "Float (single-precision)"))
  (bind _box (`self.Box`))
  (`SceneComponent.K2_AddWorldOffset` _box (* (* DeltaSeconds 5000.0) (`SceneComponent.GetForwardVector` _box)) true false))

(event `self.Cube.OnComponentBeginOverlap`
  (params (OverlappedComponent :type "PrimitiveComponent Object Reference") (OtherActor :type "Actor Object Reference") (OtherComp :type "PrimitiveComponent Object Reference") (OtherBodyIndex :type Integer) (bFromSweep :type Boolean) (SweepResult :type "HitResult Structure (by ref)"))
  (bind _returnvalue (`self.GetOwner`))
  (if (!= OtherActor _returnvalue)
    (`GameplayStatics.ApplyDamage` OtherActor 30.0 null _returnvalue)))

(event `self.ReceiveActorBeginOverlap`
  (params (OtherActor :type "Actor Object Reference"))
  (cast `/Game/1_Blueprints/BP_Enemy` OtherActor)
  (`NiagaraFunctionLibrary.SpawnSystemAtLocation` "/Game/1_Blueprints/HitPaticle.HitPaticle" (`self.K2_GetActorLocation`) (`self.K2_GetActorRotation`) (50.0 50.0 50.0))
  (`self.K2_DestroyActor`))

(fn `UserConstructionScript`)