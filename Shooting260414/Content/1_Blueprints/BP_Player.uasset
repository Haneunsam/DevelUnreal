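; Player ship pawn for a shooter that moves on the Y/Z plane with swept offsets, clamped to screen bounds deprojected from the viewport size.
; The Fire input toggles shooting, and a looping timer spawns BP_Bullet from fire points selected by the player state's Level.
; HP lives in BP_Player_State; damage lowers it, refreshes the HP bar widget and destroys the ship when depleted.
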(event `self.ReceiveTick`
  (params (DeltaSeconds :type "Float (single-precision)"))
  (bind _output_get (set `self.InputVecter` (* (`KismetMathLibrary.Normal` (`KismetMathLibrary.MakeVector` 0.0 (`self.GetInputAxisValue`) (`self.GetInputAxisValue`))) (* DeltaSeconds (`self.Speed`)))))
  (`SceneComponent.K2_AddWorldOffset` (`self.Box`) _output_get true false)
  (`self.ClampShip`))

(event `InputAxis|Forward`
  (params (AxisValue :type "Float (single-precision)")))

(event `InputAxis|rIGHT`
  (params (AxisValue :type "Float (single-precision)")))

(event `InputAction|Fire`
  (params (Key :type "Key Structure"))
  (:`Pressed`
    (set `self.IsShooting` (not (`self.IsShooting`)))))

(event `Fire`
  (if (`self.IsShooting`)
    (bind _asbp_player_state (cast `/Game/1_Blueprints/BP_Player_State` (`self.PlayerState`)))
    (for (_array_element _array_index) (`self.FireposArray`)
      (if (<= _array_index 0)
        (`self.PrimaryFire` _array_element)
        (switch `int` (`/Game/1_Blueprints/BP_Player_State.Level` _asbp_player_state)
          (:`Default`
            (`self.PrimaryFire` (`self.Firepos1`) :!label _label)
            (`self.PrimaryFire` (`self.Firepos2`) :!label _label_2))
          (:`0`
            _)
          (:`1`
            (goto _label_2))
          (:`2`
            (goto _label)))
        (`self.PrimaryFire` (`self.Firepos`))))))

(event `self.ReceiveBeginPlay`
  (bind _asbp_player_state (cast `/Game/1_Blueprints/BP_Player_State` (`GameplayStatics.GetPlayerState` 0)))
  (bind _output_get (set `/Game/1_Blueprints/BP_Player_State.MaxHP` 300.0 _asbp_player_state))
  (set `/Game/1_Blueprints/BP_Player_State.HP` _output_get _asbp_player_state)
  (`self.HPRefresh`)
  (set `self.FireposArray` (`|MakeArray` (`self.Firepos`) (`self.Firepos1`) (`self.Firepos2`)))
  (`KismetSystemLibrary.K2_SetTimerDelegate` (delegate `Fire`) 0.1 true))

(event `self.ReceiveAnyDamage`
  (params (Damage :type "Float (single-precision)") (DamageType :type "DamageType Object Reference") (InstigatedBy :type "Controller Object Reference") (DamageCauser :type "Actor Object Reference"))
  (bind _asbp_player_state (cast `/Game/1_Blueprints/BP_Player_State` (`GameplayStatics.GetPlayerState` 0)))
  (bind _returnvalue (- (`/Game/1_Blueprints/BP_Player_State.HP` _asbp_player_state) Damage))
  (set `/Game/1_Blueprints/BP_Player_State.HP` _returnvalue _asbp_player_state)
  (`self.HPRefresh`)
  (if (<= _returnvalue 0.0)
    (`self.K2_DestroyActor`)))

(event `HPRefresh`
  (bind _asbp_player_state (cast `/Game/1_Blueprints/BP_Player_State` (`GameplayStatics.GetPlayerState` 0)))
  (bind _asbp_hp_bar (cast `/Game/1_Blueprints/BP_HP_Bar` (`WidgetComponent.GetWidget` (`self.HPBar`))))
  (`ProgressBar.SetPercent` (`/Game/1_Blueprints/BP_HP_Bar.ProgressBar_32` _asbp_hp_bar) (/ (`/Game/1_Blueprints/BP_Player_State.HP` _asbp_player_state) (`/Game/1_Blueprints/BP_Player_State.MaxHP` _asbp_player_state))))

(fn `ClampShip`
  (bind _y (.y (`GameplayStatics.DeprojectScreenToWorld` (`GameplayStatics.GetPlayerController` 0) (`WidgetLayoutLibrary.GetViewportSize`))))
  (bind _z (.z (`GameplayStatics.DeprojectScreenToWorld` (`GameplayStatics.GetPlayerController` 0) (`WidgetLayoutLibrary.GetViewportSize`))))
  (`SceneComponent.K2_SetWorldLocation` (`self.Box`) (`KismetMathLibrary.MakeVector` (.x (`self.K2_GetActorLocation`)) (`KismetMathLibrary.FClamp` (.y (`self.K2_GetActorLocation`)) (* _y -1.0) _y) (`KismetMathLibrary.FClamp` (.z (`self.K2_GetActorLocation`)) _z (* _z -1.0))) false false))

(fn `PrimaryFire`
  (params (Target :type "SceneComponent Object Reference"))
  (`|SpawnActorFromClass` "/Game/1_Blueprints/BP_Bullet.BP_Bullet_C" (`SceneComponent.K2_GetComponentToWorld` Target) "Undefined" "MultiplyWithRoot" self null))

(fn `UserConstructionScript`)