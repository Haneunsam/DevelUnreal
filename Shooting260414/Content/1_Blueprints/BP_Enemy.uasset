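; BP_Enemy is an enemy actor that moves along negative world Y, damages what it overlaps and is destroyed when its health runs out.
; Tick offsets the Box component by Speed scaled by delta time, without sweeping.
; AnyDamage lowers HP and calls HPRefresh, which pushes the health ratio to the BP_HP_Bar widget's progress bar.
; Any actor overlap applies a fixed amount of damage to the other actor.
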(event `self.ReceiveBeginPlay`
  (bind _output_get (set `self.MaxHP` 100.0))
  (set `self.HP` _output_get)
  (`self.HPRefresh`))

(event `self.ReceiveTick`
  (params (DeltaSeconds :type "Float (single-precision)"))
  (`SceneComponent.K2_AddWorldOffset` (`self.Box`) (* (* DeltaSeconds (`self.speed`)) (`KismetMathLibrary.MakeVector` 0.0 -1.0)) false false))

(event `self.ReceiveAnyDamage`
  (params (Damage :type "Float (single-precision)") (DamageType :type "DamageType Object Reference") (InstigatedBy :type "Controller Object Reference") (DamageCauser :type "Actor Object Reference"))
  (set `self.HP` (- (`self.HP`) Damage))
  (`self.HPRefresh`)
  (if (<= (`self.HP`) 0.0)
    (`self.K2_DestroyActor`)))

(event `HPRefresh`
  (bind _asbp_hp_bar (cast `/Game/1_Blueprints/BP_HP_Bar` (`WidgetComponent.GetWidget` (`self.HP_Bar_0`))))
  (`ProgressBar.SetPercent` (`/Game/1_Blueprints/BP_HP_Bar.ProgressBar_32` _asbp_hp_bar) (/ (`self.HP`) (`self.MaxHP`))))

(event `self.ReceiveActorBeginOverlap`
  (params (OtherActor :type "Actor Object Reference"))
  (`GameplayStatics.ApplyDamage` OtherActor 50.0 null self))

(fn `UserConstructionScript`)